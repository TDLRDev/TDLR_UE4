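; Test tower turret that automatically tracks and shoots enemies entering its detection volume.
; Overlap events maintain a Targets list and select the oldest entry as the current target.
; Tick rotates the gun toward a lead position predicted from target velocity and projectile speed, with a Delay pacing projectile spawns at the arrow component.
; Without a valid target, the gun levels out and slowly spins.
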(event OnComponentBeginOverlap(TargetDetection)
  (params (OverlappedComponent :type Primitive%20Component%20Object%20Reference) (OtherActor :type Actor%20Object%20Reference) (OtherComp :type Primitive%20Component%20Object%20Reference) (OtherBodyIndex :type Integer) (bFromSweep :type Boolean) (SweepResult :type Hit%20Result%20Structure%20%28by%20ref%29))
  ;[1 1 1] Detect enemy and add to Targets list, set the actualTarget, First In First Attacked
  (bind (_isenemy _enemy_actor) (Enemy|IsActorEnemyProtected OtherActor))
  (if _isenemy
    (Enemy|AddEnemytoTargetsProtected _enemy_actor)
    (Enemy|SetActualTargetProtected)
    ;[0 0.6842 1] Debug
    (Development|PrintString "in")))

(event OnComponentEndOverlap(TargetDetection)
  (params (OverlappedComponent :type Primitive%20Component%20Object%20Reference) (OtherActor :type Actor%20Object%20Reference) (OtherComp :type Primitive%20Component%20Object%20Reference) (OtherBodyIndex :type Integer))
  ;[1 1 1] Detect enemy and remove from Targets list, set the actualTarget, First In First Attacked
  (bind (_isenemy _enemy_actor) (Enemy|IsActorEnemyProtected OtherActor))
  (if _isenemy
    (Enemy|RemoveEnemyfromTargetsProtected _enemy_actor)
    (Enemy|SetActualTargetProtected)
    ;[0 0.6842 1] Debug
    (Development|PrintString "out")))

(event Custom|UpdateTowerRotation
  (bind _projectileinitialspeed (Utilities|GetClassDefaults "/Game/Test/Blueprint/Abstract/Projectile/BP_ABSTRACT_Projectile.BP_ABSTRACT_Projectile_C"))
  (bind _actualtarget (Variables|Target|GetactualTarget))
  (bind _tower1_gun (Variables|Default|GetTower1_Gun))
  (bind _actualtarget_2 (Variables|Target|GetactualTarget))
  (bind _tower1_gun_2 (Variables|Default|GetTower1_Gun))
  (bind _returnvalue (Transformation|GetWorldLocation _tower1_gun_2))
  (bind _returnvalue_2 (Transformation|GetActorLocation _actualtarget))
  (bind _returnvalue_3 (Transformation|GetWorldLocation _tower1_gun))
  (bind _returnvalue_4 (Transformation|GetActorLocation _actualtarget_2))
  (bind _returnvalue_5 (Transformation|GetVelocity _actualtarget_2))
  (bind _returnvalue_6 (- _returnvalue_2 _returnvalue_3))
  (bind _returnvalue_7 (Math|Vector|VectorLength _returnvalue_6))
  (bind _returnvalue_8 (/ _returnvalue_7 _projectileinitialspeed))
  (bind _returnvalue_9 (* _returnvalue_5 _returnvalue_8))
  (bind _returnvalue_10 (+ _returnvalue_9 _returnvalue_4))
  (bind _returnvalue_11 (Math|Rotator|FindLookatRotation _returnvalue _returnvalue_10))
  (bind (_roll _pitch _yaw) (Math|Rotator|BreakRotator _returnvalue_11))
  ;[1 1 1] Tower1_Gun va target l'ennemie
  (Transformation|SetWorldRotation (Variables|Default|GetTower1_Gun) (Math|Interpolation|RInterpTo (Transformation|GetWorldRotation (Variables|Default|GetTower1_Gun)) (Math|Rotator|MakeRotator 0.0 _pitch _yaw) (Variables|Time|GetDeltaSeconds) 12.0) false false))

(event Custom|Tower%20fire
  ;[1 1 1] Tire, spawn du projectile
  (Game|SpawnActorfromClass "/Game/Test/Blueprint/Instanciable/Projectile/Test/BP_Projectile_Child.BP_Projectile_Child_C" (Transformation|GetWorldTransform (Variables|Default|GetArrow)) "Undefined" 0 0))

(event EventTick
  (params (DeltaSeconds :type Float%20%28single-precision%29))
  ;[1 0.1927 0.1927] Event Tick
  ;[1 1 1] set Delta Seconds
  (Variables|Time|SetDeltaSeconds DeltaSeconds)
  ;[1 1 1] Sequence
  (Utilities|FlowControl|Sequence
    (:then_0
      ;[1 1 1] Si enemy à target alors rotation de la tourelle vers lui sinon animation par défaut
      (if (Enemy|IsTargetValidProtected)
        (CallFunction|UpdateTowerRotation)
        (Utilities|FlowControl|Delay (/ 1.0 (Variables|Projectile|GetprojectilePerSecond)))
        (CallFunction|TowerFire)
        (else
          (Animation|IddleAnimationProtected))))))

(fn ConstructionScript)

(fn IsActorEnemyProtected
  (params (Other%20Actor :type Actor%20Object%20Reference))
  (return (Utilities|ClassIsChildOf (Utilities|GetClass Other%20Actor) "/Game/Test/Blueprint/Abstract/Enemy/BP_ABSTRACT_Enemy.BP_ABSTRACT_Enemy_C") Other%20Actor))

(fn AddEnemytoTargetsProtected
  (params (Enemy%20Actor :type Actor%20Object%20Reference))
  (if (not (Utilities|Array|ContainsItem (Variables|Target|GetTargets) Enemy%20Actor))
    (Utilities|Array|Add (Variables|Target|GetTargets) Enemy%20Actor)))

(fn RemoveEnemyfromTargetsProtected
  (params (Enemy%20Actor :type Actor%20Object%20Reference))
  (if (Utilities|Array|ContainsItem (Variables|Target|GetTargets) Enemy%20Actor)
    (Utilities|Array|RemoveItem (Variables|Target|GetTargets) Enemy%20Actor)))

(fn SetActualTargetProtected
  (Variables|Target|SetactualTarget 0)
  (if (>= (Utilities|Array|Length (Variables|Target|GetTargets)) 1)
    (Variables|Target|SetactualTarget (Utilities|Array|Get(acopy) (Variables|Target|GetTargets)))))

(fn IsTargetValidProtected
  (return (Utilities|IsValid (Variables|Target|GetactualTarget))))

(fn IddleAnimationProtected
  (bind _tower1_gun (Variables|Default|GetTower1_Gun))
  (bind _returnvalue (Transformation|GetWorldRotation _tower1_gun))
  ;[1 1 1] Comment
  (Transformation|SetWorldRotation (Variables|Default|GetTower1_Gun) (Math|Interpolation|RInterpTo _returnvalue (Math|Rotator|MakeRotator 0.0 0.0 (+ (.Yaw (Math|Rotator|BreakRotator _returnvalue)) 8.0)) (Variables|Time|GetDeltaSeconds) 5.0) false false))