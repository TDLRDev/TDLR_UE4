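; BP_ABSTRACT_Projectile is a base projectile that damages enemies it overlaps.
; Construction copies its initial speed property into the projectile movement component.
; On actor overlap, it checks that the other actor implements BPI_Damageable and derives from BP_ABSTRACT_Enemy.
; Matching actors receive DamageNumbers through the TakeDamageMessage interface call, then the projectile destroys itself; other overlaps are ignored.
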(event Collision|EventActorBeginOverlap
  (params (OtherActor :type Actor%20Object%20Reference))
  (Damage|CheckifEnemyandHitProtected OtherActor))

(fn ConstructionScript
  (Variables|/Script/Engine.ProjectileMovementComponent|SetInitialSpeed (Variables|Default|GetProjectileMovement) (Variables|Bullet_Speed|GetprojectileInitialSpeed)))

(fn CheckifEnemyandHitProtected
  (params (Other%20Actor :type Actor%20Object%20Reference))
  (if (Utilities|DoesObjectImplementInterface Other%20Actor "/Game/Test/Blueprint/Interfaces/BPI_Damageable.BPI_Damageable_C")
    (if (Utilities|ClassIsChildOf (Utilities|GetClass Other%20Actor) "/Game/Test/Blueprint/Abstract/Enemy/BP_ABSTRACT_Enemy.BP_ABSTRACT_Enemy_C")
      (Class|BPIDamageable|TakeDamage(Message) Other%20Actor (Variables|Damage|GetDamage%20Numbers))
      (Actor|DestroyActor))))