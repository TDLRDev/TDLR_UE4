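; Abstract base enemy that walks to the first BP_Nexus found at spawn and, on overlapping a Nexus, damages it by its remaining health before removing itself.
; Implements damage and destroy interface events: hits lower health and update a widget health bar, while death at zero health grants energy to the Nexus.
; Reaching the Nexus grants no energy.
; The health bar yaws toward the player camera every tick.
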(event EventBeginPlay
  ;[1 0.1927 0.1927] Event Begin Play
  (Utilities|FlowControl|Sequence
    (:then_0
      ;[1 1 1] Move actor the the Nexus
      (Movement|MoveActortoNexusProtected))
    (:then_1
      ;[1 1 1] Mise à jour de la bar de vie une première fois au spawn
      (HPBar|UpdateHPBarPercentage))))

(event EventTick
  (params (DeltaSeconds :type Float%20%28single-precision%29))
  ;[1 0.1927 0.1927] Event Tick
  ;[1 1 1] Update health bar rotation
  (HP_Bar|UpdateSceneHPBarRotationProtected))

(event EventTakeDamage
  (params (damageNumbers :type Float%20%28single-precision%29))
  ;[1 1 1] Interface Damageable
  (Damage|TakeDamageProtected damageNumbers))

(event EventDestroy
  ;[1 1 1] Interface Destroyable
  (Destroy|DestroyProtected))

(event Collision|EventActorBeginOverlap
  (params (OtherActor :type Actor%20Object%20Reference))
  ;[1 0.1927 0.1927] Event ActorBeginOverlap
  ;[1 1 1] Detection du nexus et on lui inflige des dégâts en fonction des PV actuel de l'ennemie
  (Damage|DetectandHitNexusProtected OtherActor))

(fn ConstructionScript
  ;[0.9912 0.3798 1] Construction Script
  (Utilities|FlowControl|Sequence
    (:then_0
      ;[1 1 1] On met la vie actuel au max
      (Variables|Health|SetCurrentHealth (Variables|Health|GetMaxHealth)))
    (:then_1
      ;[1 1 1] Mise à jour de la bar de vie
      (HPBar|UpdateHPBarPercentage))))

(fn GetCurrentHealth
  (return (Variables|Health|GetCurrentHealth)))

(fn GetMaxHealth
  (return (Variables|Health|GetMaxHealth)))

(fn TakeDamageProtected
  (params (DamageNumbers :type Float%20%28single-precision%29))
  ;[1 1 1] Mise à jour de la vie en fonction du nombre de dégâts
  (Variables|Default|SetcurrentHealth (- (Variables|Default|GetcurrentHealth) DamageNumbers))
  ;[1 1 1] On vérifie s'il est sur le point de mourir
  (bind _destroyed (Destroy|CanDestroyCheckProtected))
  (if (not _destroyed)
    ;[1 1 1] Si on détruit pas l'acteur on met à jour la bar de vie
    (HPBar|UpdateHPBarPercentage)))

(fn DestroyProtected
  (Energy|AddEnergytoNexus)
  (Actor|DestroyActor))

(fn MoveActortoNexusProtected
  ;[1 1 1] L'IA va vers la première instance du NEXUS
  (bind _outactors (Actor|GetAllActorsOfClass "/Game/Test/Blueprint/Instanciable/Nexus/Test/BP_Nexus.BP_Nexus_C"))
  (if (>= (Utilities|Array|Length _outactors) 1)
    (AI|Navigation|SimpleMovetoLocation (Pawn|GetController) (Transformation|GetActorLocation (Utilities|Array|Get(acopy) _outactors)))))

(fn UpdateSceneHPBarRotationProtected
  (bind _scene_hp_bar (Variables|Default|GetScene_HP_Bar))
  ;[1 0.8888 0.4989] Met à jour la rotation de la scène contenant la bar de vie en face de la camération, TODO : faire quelque chose de mieux
  (Transformation|SetWorldRotation _scene_hp_bar (Math|Rotator|MakeRotator 0.0 0.0 (.yaw (Math|Rotator|FindLookatRotation (Transformation|GetWorldLocation _scene_hp_bar) (Transformation|GetActorLocation (Game|GetPlayerCameraManager 0))))) false false))

(fn CanDestroyCheckProtected
  ;[1 1 1] Vérification de la vie, si elle est inférieur ou égale à 0 alors on détruit l'acteur
  (if (<= (Variables|Health|GetCurrentHealth) 0.0)
    (CallFunction|Destroy)
    (return true)))

(fn UpdateHPBarPercentage
  ;[1 1 1] Met à jour le poucentage de la bar de vie, Min = 0, Max = 1
  (bind _aswidget_ai_health_bar (Utilities|Casting|CastToWidget_AI_HealthBar (UserInterface|GetUserWidgetObject (Variables|Default|GetWidget_HP_Bar))))
  (Progress|SetPercent (Variables|/Game/Test/Widget/Widget_AI_HealthBar.Widget_AI_HealthBar_C|GetHealthBar _aswidget_ai_health_bar) (/ (Variables|Health|GetCurrentHealth) (Variables|Health|GetMaxHealth))))

(fn DetectandHitNexusProtected
  (params (Other%20Actor :type Actor%20Object%20Reference))
  (if (Utilities|DoesObjectImplementInterface Other%20Actor "/Game/Test/Blueprint/Interfaces/BPI_Damageable.BPI_Damageable_C")
    (if (Utilities|ClassIsChildOf (Utilities|GetClass Other%20Actor) "/Game/Test/Blueprint/Abstract/Nexus/BP_ABSTRACT_Nexus.BP_ABSTRACT_Nexus_C")
      (Class|BPIDamageable|TakeDamage(Message) Other%20Actor (Variables|Health|GetCurrentHealth))
      (Actor|DestroyActor))))

(fn AddEnergytoNexus
  (bind _outactors (Actor|GetAllActorsOfClass "/Game/Test/Blueprint/Instanciable/Nexus/Test/BP_Nexus.BP_Nexus_C"))
  (Class|BPIEnergizable|AddEnergy(Message) (Utilities|Array|Get(acopy) _outactors) (Variables|Energy|GetenergyToGive)))