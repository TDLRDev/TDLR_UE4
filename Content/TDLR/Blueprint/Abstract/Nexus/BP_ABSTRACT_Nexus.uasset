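; Abstract Nexus base Blueprint that holds clamped health and energy pools and shows a HUD widget on Begin Play.
; Damageable and Energizable interface events forward to protected functions that lower health or add and spend energy, with spending applied only when enough energy is available.
; Health starts at max in the Construction Script, and a Delay on Tick regenerates energy every second.
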(event EventTakeDamage
  (params (damageNumbers :type Float%20%28single-precision%29))
  ;[1 1 1] Interface Damageable / Fonction de dégât
  (Damage|TakeDamageProtected damageNumbers))

(event EventAddEnergy
  (params (Energy%20Numbers :type Float%20%28single-precision%29))
  ;[1 1 1] Interface Energizable
  (Energy|AddEnergyProtected Energy%20Numbers))

(event EventReduceEnergy
  (params (EnergyNumbers :type Float%20%28single-precision%29))
  ;[1 1 1] Interface Energizable
  (Energy|ReduceEnergyProtected EnergyNumbers))

(event EventBeginPlay
  ;[1 0.4582 0.4682] Event Begin Play
  ;[1 1 1] Initialisation du HUD
  (HUD|InitHUDProtected))

(event EventTick
  (params (DeltaSeconds :type Float%20%28single-precision%29))
  ;[1 0.4582 0.4682] Event Tick
  ;[1 1 1] On ajoute de l'énergie toutes les secondes
  (Utilities|FlowControl|Delay 1.0)
  (Energy|AddEnergyProtected (Variables|Energy|GetenergyToAdd)))

(fn ConstructionScript
  (Variables|Health|SetcurrentHealth (Variables|Health|GetmaxHealth)))

(fn GetCurrentHealth
  (return (Variables|Health|GetcurrentHealth)))

(fn TakeDamageProtected
  (params (DamageNumbers :type Float%20%28single-precision%29))
  (Variables|Health|SetcurrentHealth (Math|Float|Clamp(Float) (- (Variables|Health|GetcurrentHealth) DamageNumbers) 0.0 (Variables|Health|GetmaxHealth))))

(fn GetMaxHealth
  (return (Variables|Health|GetmaxHealth)))

(fn InitHUDProtected
  (bind _returnvalue (UserInterface|CreateWidget "/Game/Test/Widget/Widget_HUD.Widget_HUD_C"))
  (UserInterface|Viewport|AddtoViewport _returnvalue 0))

(fn AddEnergyProtected
  (params (EnergyNumbers :type Float%20%28single-precision%29))
  (if (< (Variables|Energy|GetcurrentEnergy) (Variables|Energy|GetmaxEnergy))
    (Variables|Energy|SetcurrentEnergy (Math|Float|Clamp(Float) (+ (Variables|Energy|GetcurrentEnergy) EnergyNumbers) 0.0 (Variables|Energy|GetmaxEnergy)))))

(fn GetCurrentEnergy
  (return (Variables|Energy|GetcurrentEnergy)))

(fn GetMaxEnergy
  (return (Variables|Energy|GetmaxEnergy)))

(fn ReduceEnergyProtected
  (params (EnergyNumbers :type Float%20%28single-precision%29))
  (if (>= (Variables|Energy|GetcurrentEnergy) EnergyNumbers)
    (Variables|Energy|SetcurrentEnergy (Math|Float|Clamp(Float) (- (Variables|Energy|GetcurrentEnergy) EnergyNumbers) 0.0 (Variables|Energy|GetmaxEnergy)))))