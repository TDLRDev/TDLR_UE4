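; Enemy spawner actor that periodically spawns AI enemies at its own transform and sends them toward the Nexus.
; Tick drives two parallel Delay-gated branches, acting as repeating timers: regular enemies on a short interval and BIG enemies on a much longer one.
; Each spawn gets a default controller, then uses SimpleMoveToLocation toward the first BP_Nexus found in the level, if one exists.
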(event EventTick
  (params (DeltaSeconds :type Float%20%28single-precision%29))
  (Utilities|FlowControl|Sequence
    (:then_0
      (Utilities|FlowControl|Delay 1.0)
      (bind _returnvalue (Game|SpawnActorfromClass "/Game/Blueprints/Instanciable/Enemy/Test/BP_Enemy.BP_Enemy_C" (Transformation|GetActorTransform) "Undefined" 0 0))
      (Pawn|SpawnDefaultController _returnvalue)
      ;[1 1 1] L'IA va vers la première instance du NEXUS
      (bind _outactors (Actor|GetAllActorsOfClass "/Game/Blueprints/Instanciable/Nexus/Test/BP_Nexus.BP_Nexus_C"))
      (if (>= (Utilities|Array|Length _outactors) 1)
        (AI|Navigation|SimpleMovetoLocation (Pawn|GetController _returnvalue) (Transformation|GetActorLocation (Utilities|Array|Get(acopy) _outactors)))))
    (:then_1
      (Utilities|FlowControl|Delay 2e+01)
      (bind _returnvalue_2 (Game|SpawnActorfromClass "/Game/Blueprints/Instanciable/Enemy/Test/BP_Enemy_BIG.BP_Enemy_BIG_C" (Transformation|GetActorTransform) "Undefined" 0 0))
      (Pawn|SpawnDefaultController _returnvalue_2)
      ;[1 1 1] L'IA va vers la première instance du NEXUS
      (bind _outactors_2 (Actor|GetAllActorsOfClass "/Game/Blueprints/Instanciable/Nexus/Test/BP_Nexus.BP_Nexus_C"))
      (if (>= (Utilities|Array|Length _outactors_2) 1)
        (AI|Navigation|SimpleMovetoLocation (Pawn|GetController _returnvalue_2) (Transformation|GetActorLocation (Utilities|Array|Get(acopy) _outactors_2)))))))

(fn ConstructionScript)