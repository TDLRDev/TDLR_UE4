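; Test tower that automatically tracks and shoots enemies entering its detection range.
; TargetDetection overlaps maintain a list of BP_ABSTRACT_Enemy actors, always targeting the earliest remaining entry.
; While the target is valid, Tick sends ABP_Sniper a look-at point led by target velocity and projectile travel time.
; A Delay based on ProjectilePerSecond paces BP_Projectile spawns from the turret's BulletSpawn socket.
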(event OnComponentBeginOverlap(TargetDetection)
  (params (OverlappedComponent :type Primitive%20Component%20Object%20Reference) (OtherActor :type Actor%20Object%20Reference) (OtherComp :type Primitive%20Component%20Object%20Reference) (OtherBodyIndex :type Integer) (bFromSweep :type Boolean) (SweepResult :type Hit%20Result%20Structure%20%28by%20ref%29))
  ;[1 1 1] Detect enemy and add to Targets list, set the actualTarget, First In First Attacked
  (bind (_isenemy _enemy_actor) (Enemy|IsActorEnemyProtected OtherActor))
  (if _isenemy
    (Enemy|AddEnemytoTargetsProtected _enemy_actor)
    (Enemy|SetActualTargetProtected)))

(event OnComponentEndOverlap(TargetDetection)
  (params (OverlappedComponent :type Primitive%20Component%20Object%20Reference) (OtherActor :type Actor%20Object%20Reference) (OtherComp :type Primitive%20Component%20Object%20Reference) (OtherBodyIndex :type Integer))
  ;[1 1 1] Detect enemy and remove from Targets list, set the actualTarget, First In First Attacked
  (bind (_isenemy _enemy_actor) (Enemy|IsActorEnemyProtected OtherActor))
  (if _isenemy
    (Enemy|RemoveEnemyfromTargetsProtected _enemy_actor)
    (Enemy|SetActualTargetProtected)))

(event Custom|UpdateTowerRotation
  (bind _actualtarget (Variables|Target|GetactualTarget))
  ;[1 1 1] Tower1_Gun va target l'ennemie
  (bind _asabp_sniper (Utilities|Casting|CastToABP_Sniper (Components|SkeletalMesh|GetAnimInstance (Variables|Default|GetTurretMesh))))
  (Variables|/Game/Models/Skeletal/Turrets/Sniper/ABP_Sniper.ABP_Sniper_C|SetLookAtLocation _asabp_sniper (+ (* (Transformation|GetVelocity _actualtarget) (/ (Math|Vector|VectorLength (- (Transformation|GetActorLocation (Variables|Target|GetactualTarget)) (Transformation|GetWorldLocation (Variables|Default|GetTurretMesh)))) (Utilities|GetClassDefaults "/Game/Blueprints/Instanciable/Projectile/Test/BP_Projectile.BP_Projectile_C"))) (Transformation|GetActorLocation _actualtarget))))

(event Custom|Tower%20fire
  ;[1 1 1] Tire, spawn du projectile
  (Game|SpawnActorfromClass "/Game/Blueprints/Instanciable/Projectile/Test/BP_Projectile.BP_Projectile_C" (Transformation|GetSocketTransform (Variables|Default|GetTurretMesh) "BulletSpawn" "RTS_World") "Undefined" 0 0))

(event EventTick
  (params (DeltaSeconds :type Float%20%28single-precision%29))
  ;[1 0.1927 0.1927] Event Tick
  ;[1 1 1] set Delta Seconds
  (Variables|Time|SetDeltaSeconds DeltaSeconds)
  ;[1 1 1] Sequence
  (Utilities|FlowControl|Sequence
    (:then_0
      ;[1 1 1] Si enemy à target alors rotation de la tourelle vers lui sinon animation par défaut
      (if (Enemy|IsTargetValidProtected)
        (CallFunction|UpdateTowerRotation)
        (Utilities|FlowControl|Delay (/ 1.0 (Variables|Projectile|GetprojectilePerSecond)))
        (CallFunction|TowerFire)))))

(fn ConstructionScript)

(fn IsActorEnemyProtected
  (params (Other%20Actor :type Actor%20Object%20Reference))
  (return (Utilities|ClassIsChildOf (Utilities|GetClass Other%20Actor) "/Game/Blueprints/Abstract/Enemy/BP_ABSTRACT_Enemy.BP_ABSTRACT_Enemy_C") Other%20Actor))

(fn AddEnemytoTargetsProtected
  (params (Enemy%20Actor :type Actor%20Object%20Reference))
  (if (not (Utilities|Array|ContainsItem (Variables|Target|GetTargets) Enemy%20Actor))
    (Utilities|Array|Add (Variables|Target|GetTargets) Enemy%20Actor)))

(fn RemoveEnemyfromTargetsProtected
  (params (Enemy%20Actor :type Actor%20Object%20Reference))
  (if (Utilities|Array|ContainsItem (Variables|Target|GetTargets) Enemy%20Actor)
    (Utilities|Array|RemoveItem (Variables|Target|GetTargets) Enemy%20Actor)))

(fn SetActualTargetProtected
  (Variables|Target|SetactualTarget 0)
  (if (>= (Utilities|Array|Length (Variables|Target|GetTargets)) 1)
    (Variables|Target|SetactualTarget (Utilities|Array|Get(acopy) (Variables|Target|GetTargets)))))

(fn IsTargetValidProtected
  (return (Utilities|IsValid (Variables|Target|GetactualTarget))))