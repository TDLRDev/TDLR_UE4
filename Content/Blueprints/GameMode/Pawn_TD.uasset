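; Player pawn (Pawn_TD) that handles movement input for a camera mounted on a spring arm.
; MoveForward and MoveRight axes feed AddMovementInput along the actor's forward and right vectors.
; A mouse-wheel zoom that would adjust the spring arm length is present but disconnected from its axis event, so it never runs.
; BeginPlay, overlap, Tick and the construction script are empty.
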(event EventBeginPlay)

(event Collision|EventActorBeginOverlap
  (params (OtherActor :type Actor%20Object%20Reference)))

(event EventTick
  (params (DeltaSeconds :type Float%20%28single-precision%29)))

(event Input|AxisEvents|InputAxisMoveForward
  (params (AxisValue :type Float%20%28single-precision%29))
  ;[1 1 1] Gestion des mouvements
  (Pawn|Input|AddMovementInput (Math|Vector|GetForwardVector (Transformation|GetActorRotation)) AxisValue false))

(event Input|AxisEvents|InputAxisMoveRight
  (params (AxisValue :type Float%20%28single-precision%29))
  ;[1 1 1] Gestion des mouvements
  (Pawn|Input|AddMovementInput (Math|Vector|GetRightVector (Transformation|GetActorRotation)) AxisValue false))

(event Input|MouseEvents|MouseWheelAxis
  (params (AxisValue :type Float%20%28single-precision%29))
  ;[1 1 1] Zoom Camera
)

(fn ConstructionScript)