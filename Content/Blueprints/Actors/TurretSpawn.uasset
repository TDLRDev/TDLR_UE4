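; Turret build spot actor that lets the player buy and place a turret by clicking.
; The construction script creates a hidden, evenly spaced preview mesh for each entry in TurretsMesh, and clicking the Cube toggles their visibility and collision.
; Clicking a preview maps its mesh index to SpawnedTurret.
; If the first BP_Nexus has 75 energy, the turret replaces the spot and that energy is deducted.
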(event OnClicked(Cube)
  (params (TouchedComponent :type Primitive%20Component%20Object%20Reference) (ButtonPressed :type Key%20Structure))
  (bind _turretshow (Variables|Default|GetTurretShow))
  (if (not (Variables|Default|Getvisibility))
    (Variables|Default|Setvisibility true)
    (Collision|SetCollisionEnabled _turretshow "QueryOnly")
    (else
      (Variables|Default|Setvisibility false)
      (Collision|SetCollisionEnabled _turretshow "NoCollision")))
  (Rendering|SetVisibility (Variables|Default|GetTurretShow) (Variables|Default|Getvisibility) false))

(event Custom|OnClicked_Event_0
  (params (TouchedComponent :type Primitive%20Component%20Object%20Reference) (ButtonPressed :type Key%20Structure))
  ;[1 1 1] Recupere l'indice de la tourelle à spawner en fonction du mesh clické
  (bind _asstatic_mesh_component (Utilities|Casting|CastToStaticMeshComponent TouchedComponent))
  ;[1 1 1] L'IA va vers la première instance du NEXUS
  (bind _outactors (Actor|GetAllActorsOfClass "/Game/Blueprints/Instanciable/Nexus/Test/BP_Nexus.BP_Nexus_C"))
  (if (>= (Variables|/Game/Blueprints/Abstract/Nexus/BP_ABSTRACT_Nexus.BP_ABSTRACT_Nexus_C|GetcurrentEnergy (Utilities|Array|Get(acopy) _outactors)) 75.0)
    ;[1 1 1] Spawn la tourelle à l'emplacement du turret spawn et destruit le turret spawner
    (Game|SpawnActorfromClass (Utilities|Array|Get(acopy) (Variables|Default|GetSpawnedTurret) (Utilities|Array|FindItem (Variables|Default|GetTurretsMesh) (Variables|/Script/Engine.StaticMeshComponent|GetStaticMesh _asstatic_mesh_component))) (Transformation|GetActorTransform) "Undefined" 0 0)
    (Actor|DestroyActor)
    (if (>= (Utilities|Array|Length _outactors) 1)
      (Class|BPIEnergizable|ReduceEnergy(Message) (Utilities|Array|Get(acopy) _outactors) 75.0))))

(event EventBeginPlay
  (EventDispatchers|AssignOnClicked (Variables|Default|GetTurretShow) (delegate Custom|OnClicked_Event_0)))

(event Collision|EventActorBeginOverlap
  (params (OtherActor :type Actor%20Object%20Reference)))

(event EventTick
  (params (DeltaSeconds :type Float%20%28single-precision%29)))

(fn ConstructionScript
  (bind _turretsmesh (Variables|Default|GetTurretsMesh))
  (for (_array_element _array_index) _turretsmesh
    ;[1 1 1] Ajoute un static mesh pour chaque tourelle selectionnable
    (bind _returnvalue (AddComponent|AddStaticMeshComponent true (Math|Transform|MakeTransform (Math|Vector|RotateVector (Utilities|NewMacro0 _array_index _turretsmesh 3e+02) "0,90.000000, 0") "0, 0, 0" "1,1,1")))
    (Rendering|SetVisibility _returnvalue false false)
    (Collision|SetCollisionEnabled _returnvalue "NoCollision")
    (Utilities|Array|AddUnique (Variables|Default|GetTurretShow) _returnvalue)
    ;[1 1 1] Bind un event click sur chaque mesh et les attach à cet acteur
    (Transformation|AttachComponentToComponent _returnvalue (Variables|Default|GetDefaultSceneRoot) "None" "KeepRelative" "KeepRelative" "KeepRelative" false)
    (Components|StaticMesh|SetStaticMesh _returnvalue _array_element)))